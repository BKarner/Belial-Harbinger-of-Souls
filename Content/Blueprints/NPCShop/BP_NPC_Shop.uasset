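; BP_NPC_Shop is an NPC shop actor that opens the shop UI and pauses the game when an AGPCharacter overlaps it.
; On overlap it takes the character's PlayerController and creates a UI_NPC_Shop widget for it, adding it to the viewport.
; The widget is cached, so later overlaps only make it visible again if hidden, then pause.
; Closing the shop and unpausing are not handled here.
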(event `self.ReceiveBeginPlay`)

(event `self.ReceiveActorBeginOverlap`
  (params (OtherActor :type "Actor Object Reference"))
  (bind _asagpcharacter (cast `AGPCharacter` OtherActor))
  (bind _returnvalue (`Controller.CastToPlayerController` (`Pawn.GetController` _asagpcharacter)))
  (set `self.Player Controller` _returnvalue)
  (`/Engine/EditorBlueprintResources/StandardMacros.IsValid` (`self.NPCShopWidget`)
    (:`Is Valid`
      (if (not (`Widget.IsVisible` (`self.NPCShopWidget`)))
        (`Widget.SetVisibility` (`self.NPCShopWidget`) "Visible")
        (`GameplayStatics.SetGamePaused` true :!label _label)))
    (:`Is Not Valid`
      (`|ExecutionSequence`
        (:`then_0`
          (bind _returnvalue_2 (`|CreateWidget` "/Game/Blueprints/NPCShop/SHOP_Widget/UI_NPC_Shop.UI_NPC_Shop_C" (`self.Player Controller`)))
          (set `self.NPCShopWidget` _returnvalue_2))
        (:`then_1`
          (`UserWidget.AddToViewport` (`self.NPCShopWidget`) 0))
        (:`then_2`
          (goto _label))))))

(event `self.ReceiveTick`
  (params (DeltaSeconds :type "Float (single-precision)")))

(fn `UserConstructionScript`)