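; BP_SavedLeaderBoards is a save game object that stores the leaderboard's ranked score list.
; IsHighScore scans the list for the first entry below a given score and returns a flag and a rank derived from that index.
; InsertScore adds an entry with an "EDIT" placeholder, trims index 6 to cap the list, then copies it into the loaded "LeaderBoard" slot save and writes it back.
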(fn `InsertScore`
  (params (Score :type "Float (double-precision)" :default 0.0) (Index :type Integer :default 0))
  (bind _score (`self.Score`))
  (`KismetArrayLibrary.Array_Insert` _score (make `/Game/Blueprints/SavedGames/SRUCT_LeaderboardScore` "EDIT" Score) Index)
  (`KismetArrayLibrary.Array_Remove` _score 6)
  (bind _returnvalue (`GameplayStatics.LoadGameFromSlot` "LeaderBoard"))
  (bind _asbp_saved_leader_boards (cast `/Game/Blueprints/SavedGames/BP_SavedLeaderBoards` _returnvalue))
  (set `/Game/Blueprints/SavedGames/BP_SavedLeaderBoards.Score` (`self.Score`) _asbp_saved_leader_boards)
  (`GameplayStatics.SaveGameToSlot` _asbp_saved_leader_boards "LeaderBoard"))

(fn `isHighScore`
  (params (Score :type "Float (double-precision)" :default 0.0))
  (returns (IsHighScore :type Boolean) (ScoreRank :type Integer))
  (for (_array_element _array_index) (`self.Score`)
    (if (< (`.LeaderBoardScore_6_D5180256434547ECD7284198B077E193` (break `/Game/Blueprints/SavedGames/SRUCT_LeaderboardScore` _array_element)) Score)
      (set `self.HighScore` true)
      (break)))
  (return (`self.HighScore`) (- _array_index 1)))