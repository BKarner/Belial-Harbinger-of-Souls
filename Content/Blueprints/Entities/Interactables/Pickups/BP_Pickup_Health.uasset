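; Health pickup that restores a set amount of health to the user who collects it, capped at their maximum.
; BeginPlay sizes the pickup sphere from PickupRange, and OnPickupPickup applies the heal once, recording the user and setting IsPickedUp.
; Tick bobs and rotates the pickup, then after collection also moves it towards the player and destroys it when MoveTowardsPlayer returns true.
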(event `self.ReceiveBeginPlay`
  ;[1 1 1] Set area for pickup
  (`SphereComponent.SetSphereRadius` (`self.pickupRange`)))

(event `self.OnPickupPickup`
  (params (User :type "PlayerCharacter Object Reference"))
  (bind _user (`self.User`))
  (set `self.User` User)
  (if (not (`self.isPickedUp`))
    (set `self.PickedUpBy` (`self.User`))
    (set `AGPCharacter.Health` (`KismetMathLibrary.FClamp` (+ (`AGPCharacter.Health` _user) (`self.GiveHealth`)) 0.0 (`AGPCharacter.MaxHealth` _user)) (`self.User`))
    (set `self.isPickedUp` true)))

(event `self.ReceiveTick`
  (params (DeltaSeconds :type "Float (single-precision)"))
  ;[1 1 1] Comment
  (`self.BobAndRotate` DeltaSeconds)
  (if (`self.isPickedUp`)
    (bind _returnvalue (`self.MoveTowardsPlayer` DeltaSeconds))
    (if _returnvalue
      (`self.K2_DestroyActor`))))

(fn `UserConstructionScript`)