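; Victory pickup that ends the game when first picked up.
; BeginPlay sizes its pickup sphere from PickupRange; on pickup it calls Victory on the AGPGame game mode, prints the user's end score and immediately quits the game.
; Tick bobs and rotates the item and, once picked up, moves it toward the player, destroying it when that move returns true.
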(event `self.ReceiveBeginPlay`
  ;[1 1 1] Set area for pickup
  (`SphereComponent.SetSphereRadius` (`self.pickupRange`)))

(event `self.OnPickupPickup`
  (params (User :type "PlayerCharacter Object Reference"))
  (set `self.User` User)
  (if (not (`self.isPickedUp`))
    (set `self.PickedUpBy` (`self.User`))
    (bind _asagpgame (cast `/Game/Blueprints/AGPGame` (`GameplayStatics.GetGameMode`)))
    (`/Game/Blueprints/AGPGame.Victory` _asagpgame)
    (set `self.isPickedUp` true)
    (`PlayerCharacter.PrintEndScore` (`self.User`))
    (`KismetSystemLibrary.QuitGame` null "Quit")))

(event `self.ReceiveTick`
  (params (DeltaSeconds :type "Float (single-precision)"))
  ;[1 1 1] Comment
  (`self.BobAndRotate` DeltaSeconds)
  (if (`self.isPickedUp`)
    (bind _returnvalue (`self.MoveTowardsPlayer` DeltaSeconds))
    (if _returnvalue
      (`self.K2_DestroyActor`))))

(fn `UserConstructionScript`)