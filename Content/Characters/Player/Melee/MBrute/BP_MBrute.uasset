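; BP_MBrute is a melee player Brute character that tracks health, attack cooldown and a score of damage dealt minus damage taken.
; Tick updates score and cooldown, while a debug fire event pulses IsFiring through a short timer.
; On death it loads or creates the LeaderBoard save, inserts qualifying high scores and opens EndScreen, removing the gameplay HUD first when a save already existed.
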(event `self.OnDeath`
  (bind _score (`self.Score`))
  (bind _score_2 (`self.Score`))
  (bind _returnvalue (`GameplayStatics.DoesSaveGameExist` "LeaderBoard"))
  (if _returnvalue
    (bind _returnvalue_2 (`GameplayStatics.LoadGameFromSlot` "LeaderBoard"))
    (bind _asbp_saved_leader_boards (cast `/Game/Blueprints/SavedGames/BP_SavedLeaderBoards` _returnvalue_2))
    (bind (_ishighscore _scorerank) (`/Game/Blueprints/SavedGames/BP_SavedLeaderBoards.isHighScore` _asbp_saved_leader_boards _score))
    (if _ishighscore
      (`/Game/Blueprints/SavedGames/BP_SavedLeaderBoards.InsertScore` _asbp_saved_leader_boards _score _scorerank))
    (bind _hud (`self.CastToBPHUD`)
      (:`Exec`
        (`/Game/HUD/UI_GameScreen.Remove` (`/Game/HUD/BP_HUD.GamePlayHUD` _hud))
        (`GameplayStatics.OpenLevel` "EndScreen")))
    (else
      (bind _returnvalue_3 (`GameplayStatics.CreateSaveGameObject` "/Game/Blueprints/SavedGames/BP_SavedLeaderBoards.BP_SavedLeaderBoards_C"))
      (`GameplayStatics.SaveGameToSlot` _returnvalue_3 "LeaderBoard")
      (bind _asbp_saved_leader_boards_2 (cast `/Game/Blueprints/SavedGames/BP_SavedLeaderBoards` _returnvalue_3))
      (bind (_ishighscore_2 _scorerank_2) (`/Game/Blueprints/SavedGames/BP_SavedLeaderBoards.isHighScore` _asbp_saved_leader_boards_2 _score_2))
      (if _ishighscore_2
        (`/Game/Blueprints/SavedGames/BP_SavedLeaderBoards.InsertScore` _asbp_saved_leader_boards_2 _score_2 _scorerank_2))
      (`GameplayStatics.OpenLevel` "EndScreen"))))

(event `self.ReceiveTick`
  (params (DeltaSeconds :type "Float (single-precision)"))
  (set `self.Score` (- (`self.DamageDone`) (`self.DamageTaken`)))
  (set `self.AttackCD` (- (`self.AttackCD`) DeltaSeconds)))

(event `self.ReceiveBeginPlay`
  (set `self.Health` (`self.MaxHealth`)))

(event `self.OnFire`
  ;[1 1 1] Debug firing
  (set `self.IsFiring?` true)
  (`KismetSystemLibrary.K2_SetTimer` null "StopFiring" 0.2))

(event `StopFiring`
  ;[1 1 1] Debug firing
  (set `self.IsFiring?` false))

(fn `UserConstructionScript`)