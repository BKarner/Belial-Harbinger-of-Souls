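; BP_RGirl is a ranged player character Blueprint that tracks health, score and firing state, and quits the game on death.
; Health starts at MaxHealth, and Tick recalculates Score as damage dealt minus damage taken while counting down the attack cooldown.
; A fire event, marked as debug, raises IsFiring and uses a short function-name timer to clear it.
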(event `self.OnDeath`
  (`KismetSystemLibrary.QuitGame` null "Quit"))

(event `self.ReceiveTick`
  (params (DeltaSeconds :type "Float (single-precision)"))
  (set `self.Score` (- (`self.DamageDone`) (`self.DamageTaken`)))
  (set `self.AttackCD` (- (`self.AttackCD`) DeltaSeconds)))

(event `self.ReceiveBeginPlay`
  (set `self.Health` (`self.MaxHealth`)))

(event `self.OnFire`
  ;[1 1 1] Debug firing
  (set `self.IsFiring?` true)
  (`KismetSystemLibrary.K2_SetTimer` null "StopFiring" 0.2))

(event `StopFiring`
  ;[1 1 1] Debug firing
  (set `self.IsFiring?` false))

(fn `UserConstructionScript`)